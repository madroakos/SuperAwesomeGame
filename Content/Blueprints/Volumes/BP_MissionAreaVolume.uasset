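; BP_MissionAreaVolume is a mission boundary volume that punishes the player for staying outside it.
; When a BP_Character leaves, it sets that character's OutsideMissionArea flag and starts a KillPlayer timer lasting SecondsToKill.
; Re-entering clears the flag and cancels the timer.
; On expiry, KillPlayer applies fixed damage to player character 0, regardless of which character left.
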(event Collision|EventActorBeginOverlap
  (params (OtherActor :type Actor%20Object%20Reference))
  (bind _asbp_character (Utilities|Casting|CastToBP_Character OtherActor))
  (Variables|/Game/Blueprints/Pawns/BP_Character.BP_Character_C|SetOutsideMissionArea _asbp_character false)
  (Utilities|Time|ClearTimerbyFunctionName 0 "KillPlayer"))

(event Collision|EventActorEndOverlap
  (params (OtherActor :type Actor%20Object%20Reference))
  (bind _asbp_character (Utilities|Casting|CastToBP_Character OtherActor))
  (Variables|/Game/Blueprints/Pawns/BP_Character.BP_Character_C|SetOutsideMissionArea _asbp_character true)
  (Utilities|Time|SetTimerbyFunctionName 0 "KillPlayer" (Variables|Default|GetSecondsToKill)))

(fn ConstructionScript)

(fn KillPlayer
  (Game|Damage|ApplyDamage (Game|GetPlayerCharacter 0) 1e+02 0 0))