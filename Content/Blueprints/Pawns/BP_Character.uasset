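; Player marine pawn for a top-down alien shooter, with world-axis movement, health, kill count, survival timer, HUD and pause menu.
; Each tick it turns control rotation toward thumbstick direction or smoothed mouse velocity, depending on the last key's device.
; Firing loops a timer-driven line trace from the rifle muzzle along control rotation, applying damage and impact effects.
; Damage triggers a low-health sound and, at zero, records run time and shows the death screen.
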(event EventBeginPlay
  (bind _asmy_game_instance (Utilities|Casting|CastToMyGameInstance (Game|GetGameInstance)))
  (Variables|Default|SetCallOfGameInstance _asmy_game_instance)
  (Variables|Timer|SetStartTime (Utilities|Time|GetGameTimeinSeconds))
  (bind _returnvalue (UserInterface|CreateWidget "/Game/UI/Menu/PauseMenu.PauseMenu_C"))
  (Variables|Default|SetPauseM _returnvalue)
  (bind _returnvalue_2 (UserInterface|CreateWidget "/Game/UI/W_PlayerHud.W_PlayerHud_C" 0 self))
  (UserInterface|Viewport|AddtoViewport _returnvalue_2 0))

(event EventTick
  (params (DeltaSeconds :type Float%20%28single-precision%29))
  ;[1 1 1] Player Aim
  (OwnFunctions|UpdatePlayerAim)
  (Timer|UpdateTime))

(event Game|Damage|EventAnyDamage
  (params (Damage :type Float%20%28single-precision%29) (DamageType :type Damage%20Type%20Object%20Reference) (InstigatedBy :type Controller%20Object%20Reference) (DamageCauser :type Actor%20Object%20Reference))
  (bind _callofgameinstance (Variables|Default|GetCallOfGameInstance))
  (if (OwnFunctions|IsAlive)
    (bind _health (OwnFunctions|DecreaseHealth Damage))
    (if (== _health 2e+01)
      (bind _returnvalue (Audio|SpawnSound2D "/Game/Sounds/InterfaceAudio/Stereo/UI_LowHealth_Loop_Stereo.UI_LowHealth_Loop_Stereo" 1.0 1.0 0.0 0))
      (elif (== _health 0.0)
        (Components|Activation|SetActive _returnvalue false false)
        (Variables|Player|SetDead true)
        (bind _returnvalue_2 (Timer|CalculateTime))
        (bind _output_get (Variables|/Game/Blueprints/MyGameInstance.MyGameInstance_C|SetEndTimeInFloat _callofgameinstance _returnvalue_2))
        (Variables|/Game/Blueprints/MyGameInstance.MyGameInstance_C|SetEndTimeInText _callofgameinstance (Utilities|Text|ToText(Float) _output_get "HalfToEven"))
        (Utilities|FlowControl|Delay 1.0)
        (bind _returnvalue_3 (UserInterface|CreateWidget "/Game/UI/DeathScreen.DeathScreen_C"))
        (UserInterface|Viewport|AddtoViewport _returnvalue_3 0)
        (if (Game|Player|IsInputKeyDown (Game|GetPlayerController 0) "LeftMouseButton")
          (Components|Activation|Deactivate (Variables|Default|GetP_AssaultRifle_MF))
          (Audio|Components|Audio|Stop (Variables|Default|GetWeaponFireSound))
          (Audio|SpawnSound2D "/Game/Sounds/Weapon_AssaultRifle/Stereo/RifleEndCue.RifleEndCue" 1.0 1.0 0.0 0))))))

(event Input|ActionEvents|InputActionFireWeapon
  (params (Key :type Key%20Structure))
  ;[1 1 1] Weapon Fire
  (:Pressed
    (Weapon|StartFiringWeapon))
  (:Released
    (Weapon|StopFiringWeapon)))

(event Input|AxisEvents|InputAxisMoveForward
  (params (AxisValue :type Float%20%28single-precision%29))
  ;[1 1 1] Input Config
  (if (OwnFunctions|IsAlive)
    (Pawn|Input|AddMovementInput "1.000000, 0, 0" AxisValue false)))

(event Input|AxisEvents|InputAxisMoveRight
  (params (AxisValue :type Float%20%28single-precision%29))
  ;[1 1 1] Input Config
  (if (OwnFunctions|IsAlive)
    (Pawn|Input|AddMovementInput "0.000000,1.000000, 0" AxisValue false)))

(event Input|KeyboardEvents|AnyKey
  (params (Key :type Key%20Structure))
  ;[1 1 1] Gamepad or Keyboard/Mouse
  (:Pressed
    (Variables|ThumbstickInput|SetGamepadActive (Class|KismetInputLibrary|KeyIsGamepadKey Key))))

(event Input|KeyboardEvents|Escape
  (params (Key :type Key%20Structure))
  (bind _returnvalue (Game|GetPlayerController 0))
  (bind _pausem (Variables|Default|GetPauseM))
  ;[1 1 1] Pause Menu
  ;;[1 1 1] Keyboard
  (:Pressed
    (Utilities|FlowControl|FlipFlop
      (:A
        (UserInterface|Viewport|AddtoViewport _pausem 0)
        (Game|SetGamePaused true)
        (Variables|/Script/Engine.PlayerController|SetbShowMouseCursor _returnvalue true)
        (Input|SetInputModeUIOnly 0 0 "LockAlways"))
      (:B
        (Widget|RemovefromParent _pausem)
        (Game|SetGamePaused false)
        (Variables|/Script/Engine.PlayerController|SetbShowMouseCursor _returnvalue false)
        (Input|SetInputModeGameOnly)))))

(event Input|GamepadEvents|GamepadSpecialRight
  (params (Key :type Key%20Structure))
  (bind _pausem (Variables|Default|GetPauseM))
  ;[1 1 1] Pause Menu
  ;;[1 1 1] Controller
  (:Pressed
    (Utilities|FlowControl|FlipFlop
      (:A
        (UserInterface|Viewport|AddtoViewport _pausem 0)
        (Game|SetGamePaused true))
      (:B
        (Widget|RemovefromParent _pausem)
        (Game|SetGamePaused false)))))

(fn ConstructionScript)

(fn UpdatePlayerAim
  (if (OwnFunctions|IsAlive)
    (if (Variables|ThumbstickInput|GetGamepadActive)
      (ThumbstickInput|UpdateThumbstickAim)
      (else
        (MouseInput|UpdateMouseAim)))))

(fn IsThumbstickAboveDeadzone
  (return (> (Math|Vector2D|Vector2DLength (Math|Vector2D|MakeVector2D (Input|AxisValues|GetThumbStickAimUp) (Input|AxisValues|GetThumbStickAimRight))) (Variables|ThumbstickInput|GetThumbStickDeadzone))))

(fn GetMouseVelocity
  (bind _returnvalue (Game|GetPlayerController 0))
  (bind (_deltax _deltay) (Class|PlayerController|GetInputMouseDelta _returnvalue))
  (return (/ (Math|Vector2D|MakeVector2D _deltax _deltay) (Utilities|Time|GetWorldDeltaSeconds))))

(fn IsMouseAboveDeadzone
  (return (> (Math|Vector2D|Vector2DLength (MouseInput|GetMouseVelocity)) (Variables|MouseInput|GetMouseDeadzone))))

(fn UpdateMouseAim
  (if (MouseInput|IsMouseAboveDeadzone)
    (Pawn|SetControlRotation (Game|GetPlayerController 0) (MouseInput|GetMouseAimDirection))))

(fn GetMouseAimDirection
  (bind _returnvalue (MouseInput|GetMouseVelocity))
  (return (Math|Interpolation|RInterpTo (Pawn|GetControlRotation (Game|GetPlayerController 0) :!class /Script/Engine.Controller) (Math|Rotator|MakeRotator 0.0 0.0 (Class|KismetMathLibrary|DegAtan2 (.x _returnvalue) (.y _returnvalue))) (Utilities|Time|GetWorldDeltaSeconds) (Variables|MouseInput|GetMouseSmoothingStrenght))))

(fn GetThumbstickAimDirection
  (return (Math|Rotator|MakeRotator 0.0 0.0 (Class|KismetMathLibrary|DegAtan2 (Input|AxisValues|GetThumbStickAimRight) (Input|AxisValues|GetThumbStickAimUp)))))

(fn UpdateThumbstickAim
  (if (ThumbstickInput|IsThumbstickAboveDeadzone)
    (Pawn|SetControlRotation (Game|GetPlayerController 0) (ThumbstickInput|GetThumbstickAimDirection))))

(fn StartFiringWeapon
  (if (OwnFunctions|IsAlive)
    (Components|Activation|Activate (Variables|Default|GetP_AssaultRifle_MF) false)
    (bind _returnvalue (Audio|SpawnSound2D "/Game/Sounds/Weapon_AssaultRifle/Stereo/RifleSoundCue.RifleSoundCue" 1.0 1.0 0.0 0))
    (Variables|Default|SetWeaponFireSound _returnvalue)
    (Weapon|WeaponTrace)
    (Utilities|Time|SetTimerbyFunctionName 0 "WeaponTrace" (Variables|Player|GetWeaponFirerate) true)))

(fn StopFiringWeapon
  (Components|Activation|Deactivate (Variables|Default|GetP_AssaultRifle_MF))
  (Audio|Components|Audio|Stop (Variables|Default|GetWeaponFireSound))
  (Utilities|Time|ClearTimerbyFunctionName 0 "WeaponTrace")
  (if (OwnFunctions|IsAlive)
    (Audio|SpawnSound2D "/Game/Sounds/Weapon_AssaultRifle/Stereo/RifleEndCue.RifleEndCue" 1.0 1.0 0.0 0)))

(fn DecreaseHealth
  (params (B :type Float%20%28single-precision%29))
  (bind _output_get (Variables|Player|SetPlayerHealth (- (Variables|Player|GetPlayerHealth) B)))
  (return _output_get))

(fn IsAlive
  (return (not (Variables|Player|GetDead))))

(fn WeaponTrace
  (bind _outhit (Collision|LineTraceByChannel (Weapon|GetWeaponTraceStartLocation) (Weapon|GetWeaponTraceEndLocation) "TraceTypeQuery1" false 0 "None"))
  (if (.bBlockingHit (Collision|BreakHitResult _outhit))
    (Game|Damage|ApplyDamage (.HitActor (Collision|BreakHitResult _outhit)) (Variables|Player|GetDamagePerShot) 0 0)
    (Weapon|SpawnImpactHit (.Location (Collision|BreakHitResult _outhit)))))

(fn GetWeaponTraceStartLocation
  (return (Transformation|GetSocketLocation (Variables|Default|GetRifle) "MuzzleFlash")))

(fn GetWeaponTraceEndLocation
  (return (+ (Weapon|GetWeaponTraceStartLocation) (* (Math|Vector|GetForwardVector (Pawn|GetControlRotation :!class /Script/Engine.Pawn)) (Variables|Player|GetWeaponRange)))))

(fn IncreaseKills
  (bind _asbp_gamemode (Utilities|Casting|CastToBP_Gamemode (Game|GetGameMode)))
  (bind _result (Math|Integer|DecrementInt (Variables|/Game/Blueprints/GameMode/BP_Gamemode.BP_Gamemode_C|GetRemainingAliensHUD _asbp_gamemode))
    (:%20%20
      (Variables|/Game/Blueprints/GameMode/BP_Gamemode.BP_Gamemode_C|SetRemainingAliensHUD _asbp_gamemode _result)
      (bind _output_get (Variables|Player|SetKills (+ (Variables|Player|GetKills) 1)))
      (return _output_get))))

(fn SpawnImpactHit
  (params (Location :type Vector))
  (Effects|SpawnEmitteratLocation "/Game/Effects/Weapons/Impacts/P_AssaultRifle_IH.P_AssaultRifle_IH" Location))

(fn AddHealth
  (params (HealthToAdd :type Float%20%28single-precision%29))
  (Variables|Player|SetPlayerHealth (Math|Float|Clamp(Float) (+ (Variables|Player|GetPlayerHealth) HealthToAdd) 0.0 1e+02)))

(fn IsHealthFull
  (return (== (Variables|Player|GetPlayerHealth) 1e+02)))

(fn CalculateTime
  (bind _output_get (Variables|Timer|SetStopTime (Utilities|Time|GetGameTimeinSeconds)))
  (return (- _output_get (Variables|Timer|GetStartTime))))

(fn UpdateTime
  (if (OwnFunctions|IsAlive)
    (bind _output_get (Timer|SetCurrentTime))
    (return _output_get)
    (else
      (return (Variables|Timer|GetCurrentTime)))))

(fn SetCurrentTime
  (bind _output_get (Variables|Timer|SetCurrentTime (- (Utilities|Time|GetGameTimeinSeconds) (Variables|Timer|GetStartTime))))
  (return _output_get))