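; Player character Blueprint for an alien shooter, holding functions for aiming, rifle fire, health, kills and survival time.
; Aim sets control yaw from either thumbstick direction or smoothed mouse velocity, each gated by a deadzone.
; Firing runs a looping timer of muzzle line traces along control rotation that apply damage and spawn impacts, alongside muzzle flash and sound.
; Kills also decrement the game mode's remaining-alien HUD counter.
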(fn ConstructionScript)

(fn UpdatePlayerAim
  (if (CallFunction|IsAlive)
    (if (Variables|Default|GetGamepadActive)
      (ThumbstickInput|UpdateThumbstickAim)
      (else
        (MouseInput|UpdateMouseAim)))))

(fn IsThumbstickAboveDeadzone
  (return (> (Math|Vector2D|Vector2DLength (Math|Vector2D|MakeVector2D (Input|AxisValues|GetThumbStickAimUp) (Input|AxisValues|GetThumbStickAimRight))) (Variables|ThumbstickInput|GetThumbStickDeadzone))))

(fn GetMouseVelocity
  (bind _returnvalue (Game|GetPlayerController 0))
  (bind (_deltax _deltay) (Class|PlayerController|GetInputMouseDelta _returnvalue))
  (return (/ (Math|Vector2D|MakeVector2D _deltax _deltay) (Utilities|Time|GetWorldDeltaSeconds))))

(fn IsMouseAboveDeadzone
  (return (> (Math|Vector2D|Vector2DLength (MouseInput|GetMouseVelocity)) (Variables|MouseInput|GetMouseDeadzone))))

(fn UpdateMouseAim
  (if (MouseInput|IsMouseAboveDeadzone)
    (Pawn|SetControlRotation (Game|GetPlayerController 0) (MouseInput|GetMouseAimDirection))))

(fn GetMouseAimDirection
  (bind _returnvalue (MouseInput|GetMouseVelocity))
  (return (Math|Interpolation|RInterpTo (Pawn|GetControlRotation (Game|GetPlayerController 0) :!class /Script/Engine.Controller) (Math|Rotator|MakeRotator 0.0 0.0 (Class|KismetMathLibrary|DegAtan2 (.x _returnvalue) (.y _returnvalue))) (Utilities|Time|GetWorldDeltaSeconds) (Variables|MouseInput|GetMouseSmoothingStrenght))))

(fn GetThumbstickAimDirection
  (return (Math|Rotator|MakeRotator 0.0 0.0 (Class|KismetMathLibrary|DegAtan2 (Input|AxisValues|GetThumbStickAimRight) (Input|AxisValues|GetThumbStickAimUp)))))

(fn UpdateThumbstickAim
  (if (ThumbstickInput|IsThumbstickAboveDeadzone)
    (Pawn|SetControlRotation (Game|GetPlayerController 0) (ThumbstickInput|GetThumbstickAimDirection))))

(fn StartFiringWeapon
  (if (CallFunction|IsAlive)
    (Components|Activation|Activate (Variables|Default|GetP_AssaultRifle_MF) false)
    (bind _returnvalue (Audio|SpawnSound2D "/Game/Sounds/Weapon_AssaultRifle/Stereo/RifleSoundCue.RifleSoundCue" 1.0 1.0 0.0 0))
    (Variables|Default|SetWeaponFireSound _returnvalue)
    (CallFunction|WeaponTrace)
    (Utilities|Time|SetTimerbyFunctionName 0 "WeaponTrace" (Variables|Default|GetWeaponFirerate) true)))

(fn StopFiringWeapon
  (Components|Activation|Deactivate (Variables|Default|GetP_AssaultRifle_MF))
  (Audio|Components|Audio|Stop (Variables|Default|GetWeaponFireSound))
  (Utilities|Time|ClearTimerbyFunctionName 0 "WeaponTrace")
  (if (CallFunction|IsAlive)
    (Audio|SpawnSound2D "/Game/Sounds/Weapon_AssaultRifle/Stereo/RifleEndCue.RifleEndCue" 1.0 1.0 0.0 0)))

(fn DecreaseHealth
  (params (B :type Float%20%28single-precision%29))
  (bind _output_get (Variables|Default|SetPlayerHealth (- (Variables|Default|GetPlayerHealth) B)))
  (return _output_get))

(fn IsAlive
  (return (not (Variables|Default|GetDead))))

(fn IsMouseButtonDown
  (if (Game|Player|IsInputKeyDown (Game|GetPlayerController 0) "LeftMouseButton")
    _))

(fn WeaponTrace
  (bind _outhit (Collision|LineTraceByChannel (CallFunction|GetWeaponTraceStartLocation) (CallFunction|GetWeaponTraceEndLocation) "TraceTypeQuery1" false 0 "None"))
  (if (.bBlockingHit (Collision|BreakHitResult _outhit))
    (Game|Damage|ApplyDamage (.HitActor (Collision|BreakHitResult _outhit)) (Variables|Default|GetDamagePerShot) 0 0)
    (CallFunction|SpawnImpactHit (.Location (Collision|BreakHitResult _outhit)))))

(fn GetWeaponTraceStartLocation
  (return (Transformation|GetSocketLocation (Variables|Default|GetRifle) "MuzzleFlash")))

(fn GetWeaponTraceEndLocation
  (return (+ (CallFunction|GetWeaponTraceStartLocation) (* (Math|Vector|GetForwardVector (Pawn|GetControlRotation :!class /Script/Engine.Pawn)) (Variables|Default|GetWeaponRange)))))

(fn IncreaseKills
  (bind _asbp_gamemode (Utilities|Casting|CastToBP_Gamemode (Game|GetGameMode)))
  (bind _result (Math|Integer|DecrementInt (Variables|/Game/Blueprints/GameMode/BP_Gamemode.BP_Gamemode_C|GetRemainingAliensHUD _asbp_gamemode))
    (:%20%20
      (Variables|/Game/Blueprints/GameMode/BP_Gamemode.BP_Gamemode_C|SetRemainingAliensHUD _asbp_gamemode _result)
      (bind _output_get (Variables|Default|SetKills (+ (Variables|Default|GetKills) 1)))
      (return _output_get))))

(fn SpawnImpactHit
  (params (Location :type Vector))
  (Effects|SpawnEmitteratLocation "/Game/Effects/Weapons/Impacts/P_AssaultRifle_IH.P_AssaultRifle_IH" Location))

(fn AddHealth
  (params (HealthToAdd :type Float%20%28single-precision%29))
  (Variables|Default|SetPlayerHealth (Math|Float|Clamp(Float) (+ (Variables|Default|GetPlayerHealth) HealthToAdd) 0.0 1e+02)))

(fn IsHealthFull
  (return (== (Variables|Default|GetPlayerHealth) 1e+02)))

(fn CalculateTime
  (bind _output_get (Variables|Default|SetStopTime (Utilities|Time|GetGameTimeinSeconds)))
  (return (- _output_get (Variables|Default|GetStartTime))))

(fn UpdateTime
  (if (CallFunction|IsAlive)
    (bind _output_get (CallFunction|SetCurrentTime))
    (return _output_get)
    (else
      (return (Variables|Default|GetCurrentTime)))))

(fn SetCurrentTime
  (bind _output_get (Variables|Default|SetCurrentTime (- (Utilities|Time|GetGameTimeinSeconds) (Variables|Default|GetStartTime))))
  (return _output_get))