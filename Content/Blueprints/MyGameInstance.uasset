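; Game instance that persists highscore name/time data across game sessions through a HighscoreSaveGame slot.
; On Init it asynchronously loads an existing save into GameInstanceArray, or creates and saves a blank one, keeping that object in CallOfSaveGame.
; On Shutdown it copies GameInstanceArray into a newly created save object and writes it asynchronously to the same slot.
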(event EventInit
  (bind _savegameslot (Variables|Default|GetSaveGameSlot))
  (bind _returnvalue (SaveGame|DoesSaveGameExist _savegameslot))
  (if _returnvalue
    (bind _savegame (|AsyncLoadGamefromSlot _savegameslot)
      (:Completed
        (bind _ashighscore_save_game (Utilities|Casting|CastToHighscoreSaveGame _savegame))
        (Variables|Default|SetGameInstanceArray (Variables|/Game/Blueprints/GameMode/HighscoreSaveGame.HighscoreSaveGame_C|GetHSNameTime _ashighscore_save_game))))
    (else
      (bind _returnvalue_2 (SaveGame|CreateSaveGameObject "/Game/Blueprints/GameMode/HighscoreSaveGame.HighscoreSaveGame_C"))
      (bind _savegame_2 (|AsyncSaveGametoSlot _returnvalue_2 _savegameslot)
        (:Completed
          (bind _ashighscore_save_game_2 (Utilities|Casting|CastToHighscoreSaveGame _savegame_2))
          (Variables|Default|SetCallOfSaveGame _ashighscore_save_game_2))))))

(event EventShutdown
  (bind _returnvalue (SaveGame|CreateSaveGameObject "/Game/Blueprints/GameMode/HighscoreSaveGame.HighscoreSaveGame_C"))
  (Variables|/Game/Blueprints/GameMode/HighscoreSaveGame.HighscoreSaveGame_C|SetHSNameTime _returnvalue (Variables|Default|GetGameInstanceArray))
  (|AsyncSaveGametoSlot _returnvalue (Variables|Default|GetSaveGameSlot)))