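; BPALien is an enemy alien pawn that chases the player and attacks up close.
; BeginPlay loops AI MoveTo with a short retry delay; Tick halts movement and plays the spider attack montage when in range, resuming on completion.
; DamagePlayer applies hit damage but is not called within this Blueprint.
; Health reaching exactly zero disables collision, credits the player's kill, notifies BP_Gamemode, then destroys the actor after a delay.
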(event EventBeginPlay
  (if true :!label _label
    (if (OwnMovement|IsAlive)
      (AI|AIMoveTo self "0, 0, 0" (Game|GetPlayerCharacter 0) 5.0 false
        (:OnSuccess
          _)
        (:OnFail
          _))
      (Utilities|FlowControl|Delay 0.2)
      (goto _label))))

(event EventTick
  (params (DeltaSeconds :type Float%20%28single-precision%29))
  (if (Attack|CanAttack)
    (OwnMovement|DeactivateAIMovement)
    (Animation|Montage|PlayMontage (Variables|Character|GetMesh) "/Game/Characters/Enemy_Great_Spider/Animations/SpiderAttack1.SpiderAttack1"
      (:OnCompleted
        (OwnMovement|ActivateAIMovement)))))

(event Game|Damage|EventAnyDamage
  (params (Damage :type Float%20%28single-precision%29) (DamageType :type Damage%20Type%20Object%20Reference) (InstigatedBy :type Controller%20Object%20Reference) (DamageCauser :type Actor%20Object%20Reference))
  (bind _health (OwnMovement|DecreaseHealth Damage))
  (if (== _health 0.0)
    (OwnMovement|KillAI)
    (Utilities|FlowControl|Delay 3.0)
    (Actor|DestroyActor)))

(fn ConstructionScript)

(fn IsWithinRange
  (return (< (Transformation|GetDistanceTo (Game|GetPlayerCharacter 0)) (LocalVariables|GetRange))))

(fn IsAttacking
  (return (Animation|Montage|MontageIsPlaying (Components|SkeletalMesh|GetAnimInstance (Variables|Character|GetMesh)) "/Game/Characters/Enemy_Great_Spider/Animations/SpiderAttack1.SpiderAttack1")))

(fn DeactivateAIMovement
  (bind _charactermovement (Variables|Character|GetCharacterMovement))
  (Components|Movement|StopMovementImmediately _charactermovement)
  (Components|Activation|Deactivate _charactermovement))

(fn ActivateAIMovement
  (Components|Activation|Activate (Variables|Character|GetCharacterMovement) false))

(fn DamagePlayer
  (if (OwnMovement|IsAlive)
    (Game|Damage|ApplyDamage (Game|GetPlayerCharacter 0) (LocalVariables|GetDamagePerHit) 0 0)))

(fn DecreaseHealth
  (params (B :type Float%20%28single-precision%29))
  (bind _output_get (Variables|OwnVariables|SetAIHealth (- (Variables|OwnVariables|GetAIHealth) B)))
  (return _output_get))

(fn KillAI
  (Variables|OwnVariables|SetDead true)
  (OwnMovement|DeactivateAIMovement)
  (Collision|SetActorEnableCollision false)
  (bind _asbp_character (Utilities|Casting|CastToBP_Character (Game|GetPlayerCharacter 0)))
  (Default|IncreaseKills _asbp_character)
  (bind _asbp_gamemode (Utilities|Casting|CastToBP_Gamemode (Game|GetGameMode)))
  (Default|RegisterAlienDeath _asbp_gamemode self))

(fn IsAlive
  (return (not (Variables|OwnVariables|GetDead))))

(fn CanAttack
  (return (Math|Boolean|ANDBoolean (Attack|IsWithinRange) (not (Attack|IsAttacking)) (OwnMovement|IsAlive))))